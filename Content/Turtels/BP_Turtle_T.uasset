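; BP_Turtle_T is an AI turtle that advances on the BP_Point_T actor and explodes there with sound and particles, destroying itself.
; BeginPlay spawns its controller, caches the target, attaches sparks and starts the chase.
; A delay-driven loop toggles the Go flag, alternating timed AIMoveTo advances toward the point with brief retreats toward BP_Nest_T, producing back-and-forth movement.
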(event `Back`
  (bind _returnvalue (`GameplayStatics.GetActorOfClass` "/Game/Nests/BP_Nest_T.BP_Nest_T_C"))
  (`|AIMoveTo` self (`SceneComponent.K2_GetComponentLocation` (`/Game/Nests/BP_Nest_T.StaticMesh` _returnvalue)) null))

(event `Chase_T`
  (bind _returnvalue (`self.K2_GetActorLocation` (`self.Point`)))
  (if (`self.Go?`)
    (`|AIMoveTo` self _returnvalue null
      (:`then`
        (`KismetSystemLibrary.Delay` 1.0)
        (set `self.Go?` false)
        (`self.Chase_T`)
        (`MovementComponent.StopMovementImmediately` (`self.CharacterMovement`))
        (`self.Back`))
      (:`OnSuccess`
        (`GameplayStatics.PlaySoundAtLocation` "/Game/StarterContent/Audio/Collapse01.Collapse01" _returnvalue (struct) 1.0 1.0 0.0 null null null null)
        (`self.K2_DestroyActor`)
        (`GameplayStatics.SpawnEmitterAtLocation` "/Game/StarterContent/Particles/P_Explosion.P_Explosion" _returnvalue (struct) (10.0 10.0 10.0))))
    (else
      (`KismetSystemLibrary.Delay` 0.5)
      (set `self.Go?` true)
      (`self.Chase_T`))))

(event `self.ReceiveBeginPlay`
  (`self.SpawnDefaultController`)
  (bind _returnvalue (`GameplayStatics.GetActorOfClass` "/Game/Points/BP_Point_T.BP_Point_T_C"))
  (set `self.Point` _returnvalue)
  (`GameplayStatics.SpawnEmitterAttached` "/Game/StarterContent/Particles/P_Sparks.P_Sparks" (`self.StaticMesh`) "None" (0.0 0.0 0.0) (struct) (10.0 10.0 10.0))
  (`self.Chase_T`))

(fn `UserConstructionScript`)