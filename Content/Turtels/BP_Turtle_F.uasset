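; BP_Turtle_F is an AI-moved turtle pawn that travels to the level's BP_Point_F and explodes on arrival.
; On BeginPlay it spawns its default controller, caches the point, attaches sparks to its Sphere and starts Chase.
; Chase uses AIMoveTo; on success it plays an explosion sound, spawns an explosion at the point and destroys itself.
; A delayed cleanup of the explosion emitter is wired after DestroyActor.
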(event `Chase`
  (bind _returnvalue (`self.K2_GetActorLocation` (`self.Point`)))
  (`|AIMoveTo` self _returnvalue null
    (:`OnSuccess`
      (`GameplayStatics.PlaySoundAtLocation` "/Game/StarterContent/Audio/Explosion01.Explosion01" (`SceneComponent.K2_GetComponentLocation` (`self.Sphere`)) (struct) 1.0 1.0 0.0 null null null null)
      (bind _returnvalue_2 (`GameplayStatics.SpawnEmitterAtLocation` "/Game/StarterContent/Particles/P_Explosion.P_Explosion" _returnvalue (struct) (10.0 10.0 10.0)))
      (`self.K2_DestroyActor`)
      (`KismetSystemLibrary.Delay` 0.2)
      (`ActorComponent.K2_DestroyComponent` _returnvalue_2))))

(event `self.ReceiveBeginPlay`
  (`self.SpawnDefaultController`)
  (bind _returnvalue (`GameplayStatics.GetActorOfClass` "/Game/Points/BP_Point_F.BP_Point_F_C"))
  (set `self.Point` _returnvalue)
  (`GameplayStatics.SpawnEmitterAttached` "/Game/StarterContent/Particles/P_Sparks.P_Sparks" (`self.Sphere`) "None" (0.0 0.0 0.0) (struct) (10.0 10.0 10.0))
  (`self.Chase`))

(fn `UserConstructionScript`)