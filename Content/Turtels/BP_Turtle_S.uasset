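; BP_Turtle_S is an AI-driven turtle character that moves in stop-and-go bursts toward the BP_Point_S actor, trailing sparks.
; On BeginPlay it spawns its controller, finds the point and starts a self-repeating chase that toggles Go.
; Each cycle runs AIMoveTo for a second, halts movement, then pauses half a second.
; A successful move plays a collapse sound, destroys the turtle and spawns a large explosion at the point.
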(event `Chase_S`
  (bind _point (`self.Point`))
  (bind _returnvalue (`self.K2_GetActorLocation` _point))
  (if (`self.Go?`)
    (`|AIMoveTo` self (0.0 0.0 0.0) _point
      (:`then`
        (`KismetSystemLibrary.Delay` 1.0)
        (set `self.Go?` false)
        (`self.Chase_S`)
        (`MovementComponent.StopMovementImmediately` (`self.CharacterMovement`)))
      (:`OnSuccess`
        (`GameplayStatics.PlaySoundAtLocation` "/Game/StarterContent/Audio/Collapse01.Collapse01" _returnvalue (struct) 1.0 1.0 0.0 null null null null)
        (`self.K2_DestroyActor`)
        (`GameplayStatics.SpawnEmitterAtLocation` "/Game/StarterContent/Particles/P_Explosion.P_Explosion" _returnvalue (struct) (10.0 10.0 10.0))))
    (else
      (`KismetSystemLibrary.Delay` 0.5)
      (set `self.Go?` true)
      (`self.Chase_S`))))

(event `self.ReceiveBeginPlay`
  (`self.SpawnDefaultController`)
  (bind _returnvalue (`GameplayStatics.GetActorOfClass` "/Game/Points/BP_Point_S.BP_Point_S_C"))
  (set `self.Point` _returnvalue)
  (`GameplayStatics.SpawnEmitterAttached` "/Game/StarterContent/Particles/P_Sparks.P_Sparks" (`self.StaticMesh`) "None" (0.0 0.0 0.0) (struct) (10.0 10.0 10.0))
  (`self.Chase_S`))

(fn `UserConstructionScript`)